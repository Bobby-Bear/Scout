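; Trigger box that streams neighbouring map sections in and out as the Scout moves through the main level.
; When BP_Scout overlaps the box, it indexes LevelStreamingArray around its SectionNumber.
; It loads and shows the sections one step either side and unloads those two steps away, all non-blocking.
; Each call runs only if that entry's soft reference resolves to a valid object.
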(event `self.Box.OnComponentBeginOverlap`
  (params (OverlappedComponent :type "PrimitiveComponent Object Reference") (OtherActor :type "Actor Object Reference") (OtherComp :type "PrimitiveComponent Object Reference") (OtherBodyIndex :type Integer) (bFromSweep :type Boolean) (SweepResult :type "HitResult Structure (by ref)"))
  (bind _levelstreamingarray (`self.LevelStreamingArray`))
  (bind _sectionnumber (`self.SectionNumber`))
  (bind _levelstreamingarray_2 (`self.LevelStreamingArray`))
  (bind _sectionnumber_2 (`self.SectionNumber`))
  (bind _output (`|GetArrayItem` _levelstreamingarray (- _sectionnumber 2)))
  (bind _output_2 (`|GetArrayItem` _levelstreamingarray (+ _sectionnumber 2)))
  (bind _output_3 (`|GetArrayItem` _levelstreamingarray_2 (+ _sectionnumber_2 1)))
  (bind _output_4 (`|GetArrayItem` _levelstreamingarray_2 (- _sectionnumber_2 1)))
  (cast `/Game/Blueprints/Character/BP_Scout_C` OtherActor)
  (`|ExecutionSequence`
    (:`then_0`
      (`/Engine/EditorBlueprintResources/StandardMacros.IsValid` (`|ConvertAsset` _output_3)
        (:`Is Valid`
          (`GameplayStatics.LoadStreamLevelBySoftObjectPtr` _output_3 true))
        (:`Is Not Valid`
          _))
      (`/Engine/EditorBlueprintResources/StandardMacros.IsValid` (`|ConvertAsset` _output_4)
        (:`Is Valid`
          (`GameplayStatics.LoadStreamLevelBySoftObjectPtr` _output_4 true))))
    (:`then_1`
      (`/Engine/EditorBlueprintResources/StandardMacros.IsValid` (`|ConvertAsset` _output_2)
        (:`Is Valid`
          (`GameplayStatics.UnloadStreamLevelBySoftObjectPtr` _output_2))
        (:`Is Not Valid`
          _))
      (`/Engine/EditorBlueprintResources/StandardMacros.IsValid` (`|ConvertAsset` _output)
        (:`Is Valid`
          (`GameplayStatics.UnloadStreamLevelBySoftObjectPtr` _output))))))

(fn `UserConstructionScript`)