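; BP_Boots is a collectible boots artifact that the Scout player picks up via interaction.
; While its gate is open, Tick shows a yaw-facing "Press key To Interact" prompt when the player is nearby, reading the bound key from Input Settings.
; ObjectInteract hides the meshes, records collection and respawn transform in the GameInstance, saves through the GameMode and plays a sound.
; It then shows fade and boots manual widgets and closes the gate, ending the prompt.
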(event `self.ReceiveTick`
  (params (DeltaSeconds :type "Float (single-precision)"))
  (bind (_returnvalue_roll _returnvalue_pitch _returnvalue_yaw) (`KismetMathLibrary.BreakRotator` (`KismetMathLibrary.FindLookAtRotation` (`self.K2_GetActorLocation`) (`self.K2_GetActorLocation` (cast `/Game/Blueprints/Character/BP_Scout_C` (`GameplayStatics.GetPlayerPawn` 0) :!pure true)))))
  (`/Engine/EditorBlueprintResources/StandardMacros.Gate` false :!label _label
    (:`Exit`
      (if (< (`KismetMathLibrary.VSize` (`KismetMathLibrary.Vector_GetAbs` (- (`self.K2_GetActorLocation`) (`self.K2_GetActorLocation` (`GameplayStatics.GetPlayerPawn` 0))))) 1000.0)
        (`TextRenderComponent.K2_SetText` (`self.Text`) (`KismetTextLibrary.Conv_StringToText` (`KismetStringLibrary.Concat_StrStr` (`KismetTextLibrary.Conv_TextToString` "Press \"") (`KismetTextLibrary.Conv_TextToString` (`KismetInputLibrary.Key_GetDisplayName` (`.Key` (break `InputActionKeyMapping` (`|GetArrayItem` (`InputSettings.GetActionMappingByName` (`InputSettings.GetInputSettings`) "Interact")))))) (`KismetTextLibrary.Conv_TextToString` "\" To Interact"))))
        (`SceneComponent.K2_SetWorldRotation` (`self.Text`) (`KismetMathLibrary.MakeRotator` 0.0 0.0 _returnvalue_yaw) false false)
        (`SceneComponent.SetVisibility` (`self.Text`) true false)
        (else
          (`SceneComponent.SetVisibility` (`self.Text`) false false))))))

(event `/Game/Blueprints/Interfaces/BP_Interact_Interface.Object Interact`
  (bind _returnvalue (`GameplayStatics.GetPlayerController` 0))
  (bind _staticmesh (`self.StaticMesh`))
  (bind _asbp_scout_c (cast `/Game/Blueprints/Character/BP_Scout_C` (`GameplayStatics.GetPlayerPawn` 0) :!pure true))
  (bind _asbp_scout_instance_gi (cast `/Game/Blueprints/Gamemodes_And_Instances/BP_ScoutInstance_GI` (`GameplayStatics.GetGameInstance`) :!pure true))
  (`|ExecutionSequence`
    (:`then_0`
      (`SceneComponent.SetVisibility` _staticmesh false false)
      (`SceneComponent.SetVisibility` (`self.StaticMesh1`) false false)
      (`PrimitiveComponent.SetCollisionEnabled` _staticmesh "NoCollision")
      (`PrimitiveComponent.SetCollisionEnabled` (`self.StaticMesh1`) "NoCollision")
      (bind _output_get (set `/Game/Blueprints/Character/BP_Scout_C.BootsCollected` true _asbp_scout_c))
      (set `/Game/Blueprints/Gamemodes_And_Instances/BP_ScoutInstance_GI.BootsCollected` _output_get _asbp_scout_instance_gi)
      (set `/Game/Blueprints/Gamemodes_And_Instances/BP_ScoutInstance_GI.LocationSpawnNew` (`self.K2_GetActorLocation` _asbp_scout_c) _asbp_scout_instance_gi)
      (set `/Game/Blueprints/Gamemodes_And_Instances/BP_ScoutInstance_GI.RotationSpawnNew` (`/Game/Blueprints/Character/BP_Scout_C.CameraRotationYaw` _asbp_scout_c) _asbp_scout_instance_gi)
      (`/Game/Blueprints/Gamemodes_And_Instances/BP_ScoutTesting_GM.Update Save` (cast `/Game/Blueprints/Gamemodes_And_Instances/BP_ScoutTesting_GM` (`GameplayStatics.GetGameMode`) :!pure true))
      (`GameplayStatics.PlaySound2D` "/Game/Audio/Milesahhh/Soundaffect/Bag-Sound_Cue.Bag-Sound_Cue" (`/Game/Blueprints/Gamemodes_And_Instances/BP_ScoutInstance_GI.Volume SFX` (cast `/Game/Blueprints/Gamemodes_And_Instances/BP_ScoutInstance_GI` (`GameplayStatics.GetGameInstance`) :!pure true)) 1.0 0.0 null null))
    (:`then_1`
      (bind _returnvalue_2 (`|CreateWidget` "/Game/Blueprints/Widgets/Transitions/Bp_BookFade_Widget.Bp_BookFade_Widget_C" _returnvalue))
      (`UserWidget.AddToViewport` _returnvalue_2 0)
      (`KismetSystemLibrary.Delay` 0.5)
      (bind _returnvalue_3 (`|CreateWidget` "/Game/Blueprints/Objects/Books/ScoutManual/BP_ScoutManualInitialBoots_Widget1.BP_ScoutManualInitialBoots_Widget1_C" _returnvalue))
      (`UserWidget.AddToViewport` _returnvalue_3 0)
      (`SceneComponent.SetVisibility` (`self.Text`) false false)
      (goto _label :!via `Close`))))

(fn `UserConstructionScript`)