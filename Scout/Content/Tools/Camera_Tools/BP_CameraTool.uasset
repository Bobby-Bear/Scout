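; BP_CameraTool is a spline camera track that flies its camera along a path and ends with a book fade widget.
; StartTrack waits briefly, then plays the MoveAlongSpline timeline at PlaybackSpeed.
; The timeline alpha sets the camera's distance along the spline and blends its rotation from StartRotation to EndRotation, independent of spline direction.
; When the timeline finishes, it creates Bp_BookFade_Widget and adds it to the viewport.
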(event `Start Track`
  (`KismetSystemLibrary.Delay` 2.0)
  (`TimelineComponent.SetPlayRate` (`self.MoveAlongSpline`) (`self.PlaybackSpeed`))
  (bind (_direction _0) (`Timeline|MoveAlongSpline` :!via `PlayFromStart`)
    (:`Update`
      (`SceneComponent.K2_SetWorldLocationAndRotation` (`self.CameraComponent`) (`SplineComponent.GetLocationAtDistanceAlongSpline` (`self.Spline`) (`KismetMathLibrary.Lerp` 0.0 (`SplineComponent.GetSplineLength` (`self.Spline`)) _0) "World") (`KismetMathLibrary.RLerp` (`self.Start Rotation`) (`self.End Rotation`) _0 true) false false))
    (:`Finished`
      (bind _returnvalue (`|CreateWidget` "/Game/Blueprints/Widgets/Transitions/Bp_BookFade_Widget.Bp_BookFade_Widget_C"))
      (`UserWidget.AddToViewport` _returnvalue 0))))

(fn `UserConstructionScript`)