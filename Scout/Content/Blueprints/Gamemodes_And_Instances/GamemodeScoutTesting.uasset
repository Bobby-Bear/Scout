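; Scout testing game mode that saves and restores player spawn and settings (sensitivity, music, SFX) through a SaveState object on ScoutGameInstance.
; After a short BeginPlay delay, UpdateSave creates and saves a default state if none exists.
; UpdateSave and SaveSettings copy game instance values into that state and write it to slot.
; Load and LoadSettings apply the in-memory state, then call LoadGameFromSlot without using its result.
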(event `self.ReceiveBeginPlay`
  (`KismetSystemLibrary.Delay` 0.2)
  (`/Engine/EditorBlueprintResources/StandardMacros.IsValid` (`/Game/Blueprints/Gamemodes_And_Instances/ScoutGameInstance.SaveState Instance` (cast `/Game/Blueprints/Gamemodes_And_Instances/ScoutGameInstance` (`GameplayStatics.GetGameInstance`) :!pure true))
    (:`Is Valid`
      (`KismetSystemLibrary.PrintString` "STATE EXISTS"))
    (:`Is Not Valid`
      (`self.Update Save`))))

(event `Load Settings`
  (bind _asscout_game_instance (cast `/Game/Blueprints/Gamemodes_And_Instances/ScoutGameInstance` (`GameplayStatics.GetGameInstance`) :!pure true))
  (bind _savestate_instance (`/Game/Blueprints/Gamemodes_And_Instances/ScoutGameInstance.SaveState Instance` _asscout_game_instance))
  (set `/Game/Blueprints/Gamemodes_And_Instances/ScoutGameInstance.Sensitivity` (`/Game/Blueprints/Gamemodes_And_Instances/SaveState.SaveSensitivity` _savestate_instance) _asscout_game_instance :!label _label)
  (set `/Game/Blueprints/Gamemodes_And_Instances/ScoutGameInstance.Volume Music` (`/Game/Blueprints/Gamemodes_And_Instances/SaveState.SaveMusic` _savestate_instance) _asscout_game_instance)
  (set `/Game/Blueprints/Gamemodes_And_Instances/ScoutGameInstance.Volume SFX` (`/Game/Blueprints/Gamemodes_And_Instances/SaveState.SaveSFX` _savestate_instance) _asscout_game_instance)
  (`KismetSystemLibrary.PrintString` "Loaded")
  (`GameplayStatics.LoadGameFromSlot` (`self.Gamemode Slot Name`)))

(event `Load`
  (bind _asbp_scout_c (cast `/Game/Blueprints/Character/BP_Scout_C` (`GameplayStatics.GetPlayerPawn` 0) :!pure true))
  (bind _savestate_instance (`/Game/Blueprints/Gamemodes_And_Instances/ScoutGameInstance.SaveState Instance` (cast `/Game/Blueprints/Gamemodes_And_Instances/ScoutGameInstance` (`GameplayStatics.GetGameInstance`) :!pure true)))
  (`self.K2_SetActorLocation` _asbp_scout_c (`/Game/Blueprints/Gamemodes_And_Instances/SaveState.SaveLocation` _savestate_instance) false false)
  (set `/Game/Blueprints/Character/BP_Scout_C.CameraRotationYaw` (`/Game/Blueprints/Gamemodes_And_Instances/SaveState.SaveRotation` _savestate_instance) _asbp_scout_c)
  (goto _label))

(event `Update Save`
  (bind _asscout_game_instance (cast `/Game/Blueprints/Gamemodes_And_Instances/ScoutGameInstance` (`GameplayStatics.GetGameInstance`) :!pure true))
  (bind _asscout_game_instance_2 (cast `/Game/Blueprints/Gamemodes_And_Instances/ScoutGameInstance` (`GameplayStatics.GetGameInstance`) :!pure true))
  (bind _savestate_instance (`/Game/Blueprints/Gamemodes_And_Instances/ScoutGameInstance.SaveState Instance` _asscout_game_instance))
  (bind _savestate_instance_2 (`/Game/Blueprints/Gamemodes_And_Instances/ScoutGameInstance.SaveState Instance` _asscout_game_instance_2))
  (`/Engine/EditorBlueprintResources/StandardMacros.IsValid` (`/Game/Blueprints/Gamemodes_And_Instances/ScoutGameInstance.SaveState Instance` (cast `/Game/Blueprints/Gamemodes_And_Instances/ScoutGameInstance` (`GameplayStatics.GetGameInstance`) :!pure true))
    (:`Is Valid`
      (set `/Game/Blueprints/Gamemodes_And_Instances/SaveState.SaveLocation` (`/Game/Blueprints/Gamemodes_And_Instances/ScoutGameInstance.LocationSpawnNew` _asscout_game_instance_2) _savestate_instance_2)
      (set `/Game/Blueprints/Gamemodes_And_Instances/SaveState.SaveRotation` (`/Game/Blueprints/Gamemodes_And_Instances/ScoutGameInstance.RotationSpawnNew` _asscout_game_instance_2) _savestate_instance_2)
      (set `/Game/Blueprints/Gamemodes_And_Instances/SaveState.SaveMusic` (`/Game/Blueprints/Gamemodes_And_Instances/ScoutGameInstance.Volume Music` _asscout_game_instance_2) _savestate_instance_2 :!label _label_2)
      (set `/Game/Blueprints/Gamemodes_And_Instances/SaveState.SaveSFX` (`/Game/Blueprints/Gamemodes_And_Instances/ScoutGameInstance.Volume SFX` _asscout_game_instance_2) _savestate_instance_2)
      (set `/Game/Blueprints/Gamemodes_And_Instances/SaveState.SaveSensitivity` (`/Game/Blueprints/Gamemodes_And_Instances/ScoutGameInstance.Sensitivity` _asscout_game_instance_2) _savestate_instance_2))
    (:`Is Not Valid`
      (bind _returnvalue (`GameplayStatics.CreateSaveGameObject` "/Game/Blueprints/Gamemodes_And_Instances/SaveState.SaveState_C"))
      (set `/Game/Blueprints/Gamemodes_And_Instances/ScoutGameInstance.SaveState Instance` _returnvalue _asscout_game_instance)
      (set `/Game/Blueprints/Gamemodes_And_Instances/SaveState.SaveLocation` (`self.PlayerLocationStart Default`) _savestate_instance)
      (set `/Game/Blueprints/Gamemodes_And_Instances/SaveState.SaveRotation` (`self.PlayerRotationStart Default`) _savestate_instance :!label _label_3)
      (set `/Game/Blueprints/Gamemodes_And_Instances/SaveState.SaveMusic` (`self.Music Default`) _savestate_instance)
      (set `/Game/Blueprints/Gamemodes_And_Instances/SaveState.SaveSFX` (`self.SFX Default`) _savestate_instance)
      (set `/Game/Blueprints/Gamemodes_And_Instances/SaveState.SaveSensitivity` (`self.Sensitivity Default`) _savestate_instance)))
  (`GameplayStatics.SaveGameToSlot` _savestate_instance (`/Game/Blueprints/Gamemodes_And_Instances/SaveState.SaveSlotName` _savestate_instance) (`/Game/Blueprints/Gamemodes_And_Instances/SaveState.UserIndex` _savestate_instance))
  (`KismetSystemLibrary.PrintString` (`KismetStringLibrary.Conv_VectorToString` (`/Game/Blueprints/Gamemodes_And_Instances/SaveState.SaveLocation` _savestate_instance)))
  (`KismetSystemLibrary.PrintString` (`KismetStringLibrary.Conv_RotatorToString` (`/Game/Blueprints/Gamemodes_And_Instances/SaveState.SaveRotation` _savestate_instance))))

(event `Save Settings`
  (`/Engine/EditorBlueprintResources/StandardMacros.IsValid` (`/Game/Blueprints/Gamemodes_And_Instances/ScoutGameInstance.SaveState Instance` (cast `/Game/Blueprints/Gamemodes_And_Instances/ScoutGameInstance` (`GameplayStatics.GetGameInstance`) :!pure true))
    (:`Is Valid`
      (goto _label_2))
    (:`Is Not Valid`
      (`GameplayStatics.CreateSaveGameObject` "/Game/Blueprints/Gamemodes_And_Instances/SaveState.SaveState_C")
      (goto _label_3))))

(fn `UserConstructionScript`)