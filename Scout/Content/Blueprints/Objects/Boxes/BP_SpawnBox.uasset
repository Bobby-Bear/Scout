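; BP_SpawnBox is a checkpoint trigger that sets a new respawn point for the Scout character.
; When a BP_Scout actor overlaps it, the box copies its Capsule's world location and rotation into that Scout's spawn variables.
; It writes the same transform to the BP_ScoutInstance_GI game instance, then calls UpdateSave on the BP_ScoutTesting_GM game mode.
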(event `self.ReceiveActorBeginOverlap`
  (params (OtherActor :type "Actor Object Reference"))
  (bind _capsule (`self.Capsule`))
  (bind _returnvalue (`SceneComponent.K2_GetComponentLocation` _capsule))
  (bind _returnvalue_2 (`SceneComponent.K2_GetComponentRotation` _capsule))
  (bind _asbp_scout_instance_gi (cast `/Game/Blueprints/Gamemodes_And_Instances/BP_ScoutInstance_GI` (`GameplayStatics.GetGameInstance`) :!pure true))
  (bind _asbp_scout_c (cast `/Game/Blueprints/Character/BP_Scout_C` OtherActor))
  (set `/Game/Blueprints/Character/BP_Scout_C.SpawnLocation` _returnvalue _asbp_scout_c)
  (set `/Game/Blueprints/Character/BP_Scout_C.SpawnRotation` _returnvalue_2 _asbp_scout_c)
  (set `/Game/Blueprints/Gamemodes_And_Instances/BP_ScoutInstance_GI.LocationSpawnNew` _returnvalue _asbp_scout_instance_gi)
  (set `/Game/Blueprints/Gamemodes_And_Instances/BP_ScoutInstance_GI.RotationSpawnNew` _returnvalue_2 _asbp_scout_instance_gi)
  (`/Game/Blueprints/Gamemodes_And_Instances/BP_ScoutTesting_GM.Update Save` (cast `/Game/Blueprints/Gamemodes_And_Instances/BP_ScoutTesting_GM` (`GameplayStatics.GetGameMode`) :!pure true)))

(fn `UserConstructionScript`)