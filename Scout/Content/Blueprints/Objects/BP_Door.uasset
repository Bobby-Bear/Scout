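; BP_Door is a keycard-locked sliding double door that opens on interact if the Scout player holds the card, which a FinalDoor consumes.
; Without the card, one indicator flashes on interact; another shows persistently, both yawed toward the player on Tick until the first opening shuts that gate.
; Timelines slide the two panels in opposite directions, with DoOnce nodes guarding open and CloseDoor.
; Closing enables Box collision and, when finished, re-arms opening.
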(event `self.ReceiveTick`
  (params (DeltaSeconds :type "Float (single-precision)"))
  (bind _asbp_scout_c (cast `/Game/Blueprints/Character/BP_Scout_C` (`GameplayStatics.GetPlayerPawn` 0) :!pure true))
  (bind (_returnvalue_roll _returnvalue_pitch _returnvalue_yaw) (`KismetMathLibrary.BreakRotator` (`KismetMathLibrary.FindLookAtRotation` (`self.K2_GetActorLocation`) (`self.K2_GetActorLocation` _asbp_scout_c))))
  (`/Engine/EditorBlueprintResources/StandardMacros.Gate` false :!label _label
    (:`Exit`
      (`SceneComponent.K2_SetWorldRotation` (`self.KeyDenied`) (`KismetMathLibrary.MakeRotator` 0.0 0.0 _returnvalue_yaw) false false)
      (`SceneComponent.K2_SetWorldRotation` (`self.KeyDenied1`) (`KismetMathLibrary.MakeRotator` 0.0 0.0 _returnvalue_yaw) false false)
      (if (`/Game/Blueprints/Character/BP_Scout_C.KeyCardCollected` _asbp_scout_c)
        (`SceneComponent.SetVisibility` (`self.KeyDenied1`) false false)
        (else
          (`SceneComponent.SetVisibility` (`self.KeyDenied1`) true false))))))

(event `self.ReceiveBeginPlay`
  (`PrimitiveComponent.SetCollisionEnabled` (`self.Box`) "NoCollision")
  (`SceneComponent.SetVisibility` (`self.KeyDenied`) false false)
  (`SceneComponent.SetVisibility` (`self.KeyDenied1`) false false))

(event `/Game/Blueprints/Interfaces/BP_Interact_Interface.Object Interact`
  (bind _asbp_scout_c (cast `/Game/Blueprints/Character/BP_Scout_C` (`GameplayStatics.GetPlayerPawn` 0) :!pure true))
  (if (`/Game/Blueprints/Character/BP_Scout_C.KeyCardCollected` _asbp_scout_c)
    (`self.OpenDoor`)
    (if (`self.FinalDoor`)
      (set `/Game/Blueprints/Character/BP_Scout_C.KeyCardCollected` false _asbp_scout_c))
    (else
      (`SceneComponent.SetVisibility` (`self.KeyDenied`) true false)
      (`KismetSystemLibrary.RetriggerableDelay` 0.5)
      (`SceneComponent.SetVisibility` (`self.KeyDenied`) false false))))

(event `OpenDoor`
  (`/Engine/EditorBlueprintResources/StandardMacros.DoOnce` false :!label _label_2
    (:`Completed`
      (`|ExecutionSequence`
        (:`then_0`
          (`SceneComponent.SetVisibility` (`self.KeyDenied1`) false false)
          (`SceneComponent.SetVisibility` (`self.KeyDenied`) false false)
          (goto _label :!via `Close`))
        (:`then_1`
          (bind (_direction _newtrack_0) (`Timeline|DoorOpen` :!via `PlayFromStart`)
            (:`Update`
              (`SceneComponent.K2_SetRelativeLocation` (`self.StaticMesh`) (* (`KismetMathLibrary.VLerp` (`self.StartLocation`) (`self.EndLocation`) _newtrack_0) -1) false false)
              (`SceneComponent.K2_SetRelativeLocation` (`self.StaticMesh1`) (`KismetMathLibrary.VLerp` (`self.StartLocation`) (`self.EndLocation`) _newtrack_0) false false))
            (:`Finished`
              (goto _label_3 :!via `Reset`))))))))

(event `ResetForTesting`
  (goto _label_2 :!via `Reset`))

(event `CloseDoor`
  (`/Engine/EditorBlueprintResources/StandardMacros.DoOnce` false :!label _label_3
    (:`Completed`
      (bind (_direction _newtrack_0) (`Timeline|Timeline_0` :!via `ReverseFromEnd`)
        (:`Update`
          (`SceneComponent.K2_SetRelativeLocation` (`self.StaticMesh`) (* (`KismetMathLibrary.VLerp` (+ (`self.StartLocation`) (-2.0 0.0 0.0)) (`self.EndLocation`) _newtrack_0) -1) false false)
          (`SceneComponent.K2_SetRelativeLocation` (`self.StaticMesh1`) (`KismetMathLibrary.VLerp` (`self.StartLocation`) (`self.EndLocation`) _newtrack_0) false false)
          (`PrimitiveComponent.SetCollisionEnabled` (`self.Box`) "QueryAndPhysics"))
        (:`Finished`
          (goto _label_2 :!via `Reset`))))))

(fn `UserConstructionScript`)