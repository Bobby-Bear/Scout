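; Grappling hook projectile for BP_Scout, trailing a cable to the player.
; In flight it aligns to its physics velocity and self-destructs after HookAirTime or on hitting anything except a BP_HookPoint.
; On a hook point it snaps, stops physics and notifies the Scout.
; The hook point's sphere radius tracks rope length: sized on attach, adjusted by MoveOneRope, reset when the hook is destroyed.
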(event `self.ReceiveBeginPlay`
  (add `/Game/Blueprints/Gamemodes_And_Instances/BP_ScoutInstance_GI.SFX Volume Changed` (cast `/Game/Blueprints/Gamemodes_And_Instances/BP_ScoutInstance_GI` (`GameplayStatics.GetGameInstance`) :!pure true) (delegate `SFX Changed`)))

(event `SFX Changed`
  (params (NewValue :type "Float (double-precision)"))
  (set `self.SFX Volume` NewValue))

(event `MoveOneRope`
  (params (VerticalMovement :type Integer) (Distance :type "Float (double-precision)"))
  (if (`/Game/Blueprints/Character/BP_Scout_C.HookIsAttached` (cast `/Game/Blueprints/Character/BP_Scout_C` (`self.Player`) :!pure true))
    (bind _sphere (`/Game/Blueprints/Objects/BP_HookPoint.Sphere` (stale `self.Sphere.OnComponentHit` _asbp_hook_point)))
    (`SphereComponent.SetSphereRadius` _sphere (`KismetMathLibrary.Abs` (- (`SphereComponent.SphereRadius` _sphere) (* VerticalMovement Distance))) true)))

(event `GetPlayer`
  (params (Player :type "Character Object Reference"))
  (bind _output_get (set `self.Player` Player))
  (`CableComponent.SetAttachEndTo` (`self.Cable`) _output_get "None" "None"))

(event `self.ReceiveDestroyed`
  (`/Engine/EditorBlueprintResources/StandardMacros.IsValid` (stale `self.Sphere.OnComponentHit` _asbp_hook_point)
    (:`Is Valid`
      (`SphereComponent.SetSphereRadius` (`/Game/Blueprints/Objects/BP_HookPoint.Sphere` (stale `self.Sphere.OnComponentHit` _asbp_hook_point)) 90.0 true))))

(event `self.Sphere.OnComponentHit`
  (params (HitComponent :type "PrimitiveComponent Object Reference") (OtherActor :type "Actor Object Reference") (OtherComp :type "PrimitiveComponent Object Reference") (NormalImpulse :type "Vector Structure") (Hit :type "HitResult Structure (by ref)"))
  (bind _returnvalue (`self.K2_GetActorLocation`))
  (bind _returnvalue_2 (`KismetMathLibrary.Vector_Distance` (`self.K2_GetActorLocation` (`self.Player`)) (`self.K2_GetActorLocation`)))
  (bind _asbp_hook_point (cast `/Game/Blueprints/Objects/BP_HookPoint` OtherActor)
    (:`then`
      (`self.K2_SetActorLocation` (`self.K2_GetActorLocation` _asbp_hook_point))
      (`PrimitiveComponent.SetSimulatePhysics` (`self.Sphere`) false)
      (set `CableComponent.CableLength` (/ _returnvalue_2 2.0) (`self.Cable`))
      (`SphereComponent.SetSphereRadius` (`/Game/Blueprints/Objects/BP_HookPoint.Sphere` _asbp_hook_point) (+ _returnvalue_2 50.0) true)
      (`/Game/Blueprints/Character/BP_Scout_C.HookAttached` (cast `/Game/Blueprints/Character/BP_Scout_C` (`self.Player`) :!pure true) _returnvalue)
      (`GameplayStatics.PlaySoundAtLocation` null _returnvalue (struct) (`self.SFX Volume`) 1.0 0.0 null null null))
    (:`CastFailed`
      (`self.K2_DestroyActor`)
      (set `/Game/Blueprints/Character/BP_Scout_C.HookIsAttached` false (cast `/Game/Blueprints/Character/BP_Scout_C` (`self.Player`) :!pure true)))))

(event `self.ReceiveTick`
  (params (DeltaSeconds :type "Float (single-precision)"))
  (bind _returnvalue (+ DeltaSeconds (`self.Seconds`)))
  (if (`/Game/Blueprints/Character/BP_Scout_C.HookIsAttached` (cast `/Game/Blueprints/Character/BP_Scout_C` (`self.Player`) :!pure true))
    (set `self.Seconds` 1.0)
    (`/Game/Blueprints/Character/BP_Scout_C.HookAttached` (cast `/Game/Blueprints/Character/BP_Scout_C` (`self.Player`) :!pure true) (`self.K2_GetActorLocation`))
    (else
      (set `self.SwingSeconds` _returnvalue)
      (bind _output_get (set `self.Seconds` _returnvalue))
      (if (< _output_get (`self.HookAirTime`))
        (bind _returnvalue_2 (`PrimitiveComponent.GetPhysicsLinearVelocity` (`self.Sphere`) "None"))
        (bind (_returnvalue_roll _returnvalue_pitch _returnvalue_yaw) (`KismetMathLibrary.BreakRotator` (`KismetMathLibrary.Conv_VectorToRotator` _returnvalue_2)))
        (`self.K2_SetActorRotation` (`KismetMathLibrary.MakeRotator` _returnvalue_roll (+ _returnvalue_pitch 90.0) _returnvalue_yaw))
        (else
          (`self.K2_DestroyActor`)
          (set `self.Seconds` 0.0)
          (set `/Game/Blueprints/Character/BP_Scout_C.HookIsAttached` false (cast `/Game/Blueprints/Character/BP_Scout_C` (`self.Player`) :!pure true)))))))

(fn `UserConstructionScript`)