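; BP_Robot is an interactable robot NPC that plays voice lines at the start or, with RobotEnd set, receives the player's artifact and ends the game.
; Tick loops bobble and head-turn timelines through DoOnce resets, optionally faces the player, shows a proximity prompt and keeps the given artifact bobbing along.
; Gates sequence interaction: the ending robot flies in, takes the artifact, closes its door, departs and opens the credits transition.
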(event `self.ReceiveTick`
  (params (DeltaSeconds :type "Float (single-precision)"))
  (bind _door (`self.Door`))
  (bind _head (`self.Head`))
  (bind _head_2 (`self.Head`))
  (bind _artifact (`self.Artifact`))
  (bind _artifact_2 (`self.Artifact`))
  (bind _returnvalue (`SceneComponent.K2_GetComponentRotation` (`self.Body`)))
  (bind _roll (.roll _returnvalue))
  (bind _pitch (.pitch _returnvalue))
  (bind _yaw (.yaw _returnvalue))
  (bind (_returnvalue_roll _returnvalue_pitch _returnvalue_yaw) (`KismetMathLibrary.BreakRotator` (`KismetMathLibrary.FindLookAtRotation` (`self.K2_GetActorLocation`) (`self.K2_GetActorLocation` (cast `/Game/Blueprints/Character/BP_Scout_C` (`GameplayStatics.GetPlayerPawn` 0) :!pure true)))))
  (bind (_returnvalue_roll_2 _returnvalue_pitch_2 _returnvalue_yaw_2) (`KismetMathLibrary.BreakRotator` (`KismetMathLibrary.FindLookAtRotation` (`self.K2_GetActorLocation`) (`self.K2_GetActorLocation` (cast `/Game/Blueprints/Character/BP_Scout_C` (`GameplayStatics.GetPlayerPawn` 0) :!pure true)))))
  (`|ExecutionSequence`
    (:`then_0`
      ;[1 1 1] Bobble
      (if (not (`self.DoNotBobble`))
        (`/Engine/EditorBlueprintResources/StandardMacros.DoOnce` false :!label _label
          (:`Completed`
            (bind (_direction _newtrack_0) (`Timeline|Bobble` :!via `PlayFromStart`)
              (:`Update`
                (if (>= _newtrack_0 0.0)
                  (bind _returnvalue_2 (`KismetMathLibrary.VLerp` (`self.BobbleStart`) (`self.BobbleEnd`) _newtrack_0))
                  (`SceneComponent.K2_SetRelativeLocation` (`self.Body`) _returnvalue_2 false false)
                  (`SceneComponent.K2_SetRelativeLocation` _head (+ _returnvalue_2 (0.0 0.0 100.0)) false false)
                  (`SceneComponent.K2_SetRelativeLocation` _door (+ _returnvalue_2 (50.0 0.0 0.0)) false false)
                  (set `self.ArtifactBobble` _returnvalue_2)
                  (else
                    (bind _returnvalue_3 (* _returnvalue_2 -1.0))
                    (`SceneComponent.K2_SetRelativeLocation` (`self.Door`) _returnvalue_3 false false)
                    (`SceneComponent.K2_SetRelativeLocation` (`self.Head`) _returnvalue_3 false false)
                    (`SceneComponent.K2_SetRelativeLocation` (`self.Body`) _returnvalue_3 false false)
                    (`SceneComponent.K2_SetRelativeLocation` _head (+ _returnvalue_3 (0.0 0.0 100.0)) false false)
                    (`SceneComponent.K2_SetRelativeLocation` _door (+ _returnvalue_3 (50.0 0.0 0.0)) false false)
                    (set `self.ArtifactBobble` _returnvalue_3))))
              (:`Finished`
                (`self.ReloopBobble`)))))))
    (:`then_1`
      ;[1 1 1] Rotate Head
      (`/Engine/EditorBlueprintResources/StandardMacros.DoOnce` false :!label _label_2
        (:`Completed`
          (bind (_direction_2 _newtrack_0_2) (`Timeline|HeadTurn` :!via `PlayFromStart`)
            (:`Update`
              (if (>= _newtrack_0_2 0.0)
                (`SceneComponent.K2_SetWorldRotation` _head_2 (`KismetMathLibrary.RLerp` _returnvalue (`KismetMathLibrary.MakeRotator` _roll _pitch (+ _yaw 30.0)) _newtrack_0_2) false false)
                (else
                  (`SceneComponent.K2_SetWorldRotation` _head_2 (`KismetMathLibrary.RLerp` _returnvalue (`KismetMathLibrary.MakeRotator` _roll _pitch (- _yaw 30.0)) _newtrack_0_2) false false))))
            (:`Finished`
              (`self.Reset HeadTurn`))))))
    (:`then_2`
      ;[1 1 1] FaceTowardPlayer
      (if (`self.FaceTowardPlayer`)
        (`self.K2_SetActorRotation` (`KismetMathLibrary.MakeRotator` 0.0 0.0 _returnvalue_yaw_2))))
    (:`then_3`
      (`/Engine/EditorBlueprintResources/StandardMacros.Gate` true :!label _label_3
        (:`Exit`
          (`/Engine/EditorBlueprintResources/StandardMacros.IsValid` _artifact_2
            (:`Is Valid`
              (`self.K2_SetActorLocation` _artifact_2 (+ (`self.ArtifactBobble`) (- (`self.K2_GetActorLocation`) (-16.0 5.0 110.0))) false false)
              (`KismetSystemLibrary.PrintString` "Hello"))))))
    (:`then_5`
      ;[1 1 1] Text
      (if (`self.VisibleText`)
        (`/Engine/EditorBlueprintResources/StandardMacros.Gate` false :!label _label_4
          (:`Exit`
            (if (< (`KismetMathLibrary.VSize` (`KismetMathLibrary.Vector_GetAbs` (- (`self.K2_GetActorLocation`) (`self.K2_GetActorLocation` (`GameplayStatics.GetPlayerPawn` 0))))) 1000.0)
              (`TextRenderComponent.K2_SetText` (`self.Text`) (`KismetTextLibrary.Conv_StringToText` (`KismetStringLibrary.Concat_StrStr` (`KismetTextLibrary.Conv_TextToString` "Press \"") (`KismetTextLibrary.Conv_TextToString` (`KismetInputLibrary.Key_GetDisplayName` (`.Key` (break `InputActionKeyMapping` (`|GetArrayItem` (`InputSettings.GetActionMappingByName` (`InputSettings.GetInputSettings`) "Interact")))))) (`KismetTextLibrary.Conv_TextToString` "\" To Interact"))))
              (`SceneComponent.K2_SetWorldRotation` (`self.Text`) (`KismetMathLibrary.MakeRotator` 0.0 0.0 _returnvalue_yaw) false false)
              (`SceneComponent.SetVisibility` (`self.Text`) true false)
              (else
                (`SceneComponent.SetVisibility` (`self.Text`) false false)))))))
    (:`then_6`
      (`/Engine/EditorBlueprintResources/StandardMacros.IsValid` _artifact
        (:`Is Valid`
          (if (`/Game/Blueprints/Objects/Artifacts/BP_Artifact.Attatched` _artifact)
            (`/Engine/EditorBlueprintResources/StandardMacros.Gate` true :!label _label_5
              (:`Exit`
                (`/Engine/EditorBlueprintResources/StandardMacros.DoOnce` false
                  (:`Completed`
                    (set `self.VisibleText` false)))))))))))

(event `ReloopBobble`
  ;[1 1 1] Bobble
  (goto _label :!via `Reset`))

(event `Reset HeadTurn`
  ;[1 1 1] Rotate Head
  (goto _label_2 :!via `Reset`))

(event `CloseRobotDoor`
  (bind _artifact (`self.Artifact`))
  (bind _artifact_2 (`self.Artifact`))
  ;[1 1 1] Open Door
  (bind (_direction _newtrack_0) (`Timeline|DoorOpen` :!via `ReverseFromEnd` :!label _label_6)
    (:`Update`
      (`SceneComponent.K2_SetRelativeRotation` (`self.Door`) (`KismetMathLibrary.RLerp` (struct :`Pitch` 30.0 :`Yaw` 180.0) (struct :`Pitch` 210.0 :`Yaw` 180.0) _newtrack_0) false false)
      (goto _label_5 :!via `Open`))
    (:`Finished`
      (goto _label_7 :!via `Open`))))

(event `self.ReceiveBeginPlay`
  (`SceneComponent.K2_SetWorldRotation` (`self.Door`) (`self.DefaultDoorRotation`) false false)
  (`KismetSystemLibrary.Delay` 0.1)
  (if (`self.RobotEnd`)
    (bind (_direction _newtrack_1) (`Timeline|BeginningSpawn` :!via `PlayFromStart`)
      (:`Update`
        (`self.K2_SetActorLocation` (+ (`KismetMathLibrary.VLerp` (`self.RobotEndBeginning`) (`self.RobotStartBeginning`) _newtrack_1) (`self.SpawnLocation`))))
      (:`Finished`
        (`|ExecutionSequence`
          (:`then_0`
            ;[1 1 1] Open Door
            (`/Engine/EditorBlueprintResources/StandardMacros.DoOnce` false
              (:`Completed`
                (goto _label_6))))
          (:`then_1`
            (goto _label_8 :!via `Open`)))))))

(event `Robot Loaded`
  (bind _asbp_scout_instance_gi (cast `/Game/Blueprints/Gamemodes_And_Instances/BP_ScoutInstance_GI` (`GameplayStatics.GetGameInstance`)))
  (`GameplayStatics.PlaySoundAtLocation` "/Game/Audio/Voicelines/Robot/RobotBeginning_0.RobotBeginning_0" (`self.K2_GetActorLocation`) (struct) (`/Game/Blueprints/Gamemodes_And_Instances/BP_ScoutInstance_GI.Volume SFX` _asbp_scout_instance_gi) 1.0 0.0 null null null)
  (`GameplayStatics.PlaySoundAtLocation` "/Game/Audio/Milesahhh/Soundaffect/Space-Ship-Landing-Sound_Cue.Space-Ship-Landing-Sound_Cue" (`self.K2_GetActorLocation`) (struct) 1.0 1.0 0.0 null null null)
  (`SceneComponent.SetVisibility` (`self.Text`) false false)
  (`SceneComponent.K2_SetRelativeRotation` (`self.Door`) (struct :`Pitch` 30.0 :`Yaw` 180.0) false false)
  (`KismetSystemLibrary.Delay` 9.0)
  (goto _label_10 :!via `Reset`))

(event `/Game/Blueprints/Interfaces/BP_Interact_Interface.Object Interact`
  (bind _artifact (`self.Artifact`))
  (bind _artifact_2 (`self.Artifact`))
  (if (`self.RobotEnd`)
    (`/Engine/EditorBlueprintResources/StandardMacros.Gate` true :!label _label_7
      (:`Exit`
        (`/Engine/EditorBlueprintResources/StandardMacros.IsValid` _artifact
          (:`Is Valid`
            (if (`/Game/Blueprints/Objects/Artifacts/BP_Artifact.Attatched` _artifact)
              (`|ExecutionSequence`
                (:`then_0`
                  (goto _label_9 :!via `Close`))
                (:`then_1`
                  (set `/Game/Blueprints/Objects/Artifacts/BP_Artifact.Attatched` false _artifact)
                  (`|ExecutionSequence`
                    (:`then_0`
                      (`/Game/Blueprints/Character/BP_Scout_C.ArtifactGiven` (cast `/Game/Blueprints/Character/BP_Scout_C` (`GameplayStatics.GetPlayerPawn` 0) :!pure true))
                      (set `/Game/Blueprints/Objects/Artifacts/BP_Artifact.RobotGiven` true _artifact_2)
                      (`self.SetActorScale3D` _artifact_2 (1.0 1.0 1.0))
                      (`self.CloseRobotDoor`)
                      (`/Engine/EditorBlueprintResources/StandardMacros.Gate` true :!label _label_8
                        (:`Exit`
                          (goto _label_3 :!via `Open`))))
                    (:`then_1`
                      (`SceneComponent.SetVisibility` (`self.Text`) false false)
                      (bind _asbp_scout_instance_gi (cast `/Game/Blueprints/Gamemodes_And_Instances/BP_ScoutInstance_GI` (`GameplayStatics.GetGameInstance`)))
                      (bind _volume_sfx (`/Game/Blueprints/Gamemodes_And_Instances/BP_ScoutInstance_GI.Volume SFX` _asbp_scout_instance_gi))
                      (`GameplayStatics.PlaySound2D` "/Game/Audio/Voicelines/Robot/RobotEnding_1.RobotEnding_1" _volume_sfx 1.0 0.0 null null)
                      (`KismetSystemLibrary.Delay` 2.5)
                      (`GameplayStatics.PlaySound2D` "/Game/Audio/Voicelines/Robot/RobotEnding_2.RobotEnding_2" _volume_sfx 1.0 0.0 null null)
                      (`KismetSystemLibrary.Delay` 5.0)
                      (set `self.DoNotBobble` true)
                      (set `self.StartPointEnd` (`self.K2_GetActorLocation`))
                      (bind _outactors (`GameplayStatics.GetAllActorsOfClass` "/Game/Blueprints/Objects/Boxes/BP_TemporaryBox.BP_TemporaryBox_C"))
                      (set `/Game/Blueprints/Objects/Boxes/BP_TemporaryBox.Collision` false (`|GetArrayItem` _outactors))
                      (bind (_direction _newtrack_0) (`Timeline|Timeline_0` :!via `PlayFromStart`)
                        (:`Update`
                          (`self.K2_SetActorLocation` (+ (`KismetMathLibrary.VLerp` (`self.RobotStartFinal`) (`self.RobotEndFinal`) _newtrack_0) (`self.StartPointEnd`)))
                          (if (> _newtrack_0 0.1)
                            (`/Engine/EditorBlueprintResources/StandardMacros.DoOnce` false
                              (:`Completed`
                                (set `/Game/Blueprints/Character/BP_Scout_C.MusicSelect` 6 (cast `/Game/Blueprints/Character/BP_Scout_C` (`GameplayStatics.GetPlayerPawn` 0) :!pure true))))))
                        (:`Finished`
                          (bind _returnvalue (`|CreateWidget` "/Game/Blueprints/Widgets/Widget_HUD/BP_CreditsTransition.BP_CreditsTransition_C"))
                          (set `/Game/Blueprints/Widgets/Widget_HUD/BP_CreditsTransition.Robot` self _returnvalue)
                          (`UserWidget.AddToViewport` _returnvalue 0)))))))
              (else
                (`/Engine/EditorBlueprintResources/StandardMacros.Gate` true :!label _label_9
                  (:`Exit`
                    (`/Engine/EditorBlueprintResources/StandardMacros.DoOnce` false
                      (:`Completed`
                        (bind _asbp_scout_instance_gi_2 (cast `/Game/Blueprints/Gamemodes_And_Instances/BP_ScoutInstance_GI` (`GameplayStatics.GetGameInstance`)))
                        (`GameplayStatics.PlaySoundAtLocation` "/Game/Audio/Voicelines/Robot/RobotEnding_0.RobotEnding_0" (`self.K2_GetActorLocation`) (struct) (`/Game/Blueprints/Gamemodes_And_Instances/BP_ScoutInstance_GI.Volume SFX` _asbp_scout_instance_gi_2) 1.0 0.0 null null null)))))))))))
    (elif (not (`/Game/Blueprints/Gamemodes_And_Instances/BP_ScoutInstance_GI.Resume` (cast `/Game/Blueprints/Gamemodes_And_Instances/BP_ScoutInstance_GI` (`GameplayStatics.GetGameInstance`) :!pure true)))
      (`/Engine/EditorBlueprintResources/StandardMacros.DoOnce` true :!label _label_10
        (:`Completed`
          (`|ExecutionSequence`
            (:`then_0`
              ;[1 1 1] Text
              (`SceneComponent.SetVisibility` (`self.Text`) false false)
              (goto _label_4 :!via `Close`))
            (:`then_1`
              (bind _asbp_scout_instance_gi_3 (cast `/Game/Blueprints/Gamemodes_And_Instances/BP_ScoutInstance_GI` (`GameplayStatics.GetGameInstance`)))
              (`GameplayStatics.PlaySoundAtLocation` (select `int` (`KismetMathLibrary.RandomIntegerInRange` 0 1) :`0` "/Game/Audio/Voicelines/Robot/RobotBeginning_1.RobotBeginning_1" :`1` "/Game/Audio/Voicelines/Robot/RobotBeginning_0.RobotBeginning_0" :!type "SoundBase Object Reference") (`self.K2_GetActorLocation`) (struct) (`/Game/Blueprints/Gamemodes_And_Instances/BP_ScoutInstance_GI.Volume SFX` _asbp_scout_instance_gi_3) 1.0 0.0 null null null)
              (`KismetSystemLibrary.Delay` 6.0)
              (`|ExecutionSequence`
                (:`then_0`
                  (goto _label_10 :!via `Reset`))
                (:`then_1`
                  (goto _label_4 :!via `Open`))))))))))

(event `Start Credits`
  (`self.Credits`))

(fn `UserConstructionScript`)