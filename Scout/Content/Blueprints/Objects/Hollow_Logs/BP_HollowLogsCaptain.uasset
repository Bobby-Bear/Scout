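; BP_HollowLogsCaptain is an interactable log object that plays a voiced, subtitled dialogue sequence.
; On interact, Tick reads numbered rows from the DataTable selected by HollowLogInteger, showing text yawed toward the Scout and playing sound.
; Each row's Time delays the next line via a DoOnce reset; a missing row hides the text and rewinds.
; While inactive, a second billboard blinks on a one-second timer as an indicator.
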(event `self.ReceiveBeginPlay`
  (`SceneComponent.SetVisibility` (`self.TextRender`) false true)
  (`SceneComponent.SetVisibility` (`self.MaterialBillboard`) false true))

(event `self.ReceiveTick`
  (params (DeltaSeconds :type "Float (single-precision)"))
  (set `self.Delta Seconds` DeltaSeconds)
  (if (`self.Activate`)
    (`/Engine/EditorBlueprintResources/StandardMacros.Gate` true :!label _label
      (:`Exit`
        (`self.RotationToPlayer`)
        (bind _returnvalue (`|GetDataTableRow` (`|GetArrayItem` (`self.HollowLogs DT Array`) (`self.HollowLog Integer`)) (`KismetStringLibrary.Conv_StringToName` (`KismetStringLibrary.Conv_IntToString` (`self.LineNumber`))))
          (:`then`
            (bind (_dialogueline _sound _time) (break `/Game/Blueprints/Objects/Hollow_Logs/Structure_Hollowlogs` _returnvalue))
            (`TextRenderComponent.K2_SetText` (`self.TextRender`) _dialogueline)
            (`/Engine/EditorBlueprintResources/StandardMacros.DoOnce` false :!label _label_2
              (:`Completed`
                (`GameplayStatics.PlaySound2D` _sound 1.0 1.0 0.0 null null false)
                (`self.Hollowlog Cycle` _time))))
          (:`RowNotFound`
            (`SceneComponent.SetVisibility` (`self.TextRender`) false false)
            (`SceneComponent.SetVisibility` (`self.MaterialBillboard`) false false)
            (`KismetSystemLibrary.PrintString` "NOOOOOOO")
            (set `self.Activate` false)
            (set `self.LineNumber` 1)
            (goto _label :!via `Close`)))))
    (else
      (set `self.FlipflopTimer` (+ (`self.Delta Seconds`) (`self.FlipflopTimer`)))
      (`|ExecutionSequence`
        (:`then_0`
          (`/Engine/EditorBlueprintResources/StandardMacros.DoOnce` false :!label _label_3
            (:`Completed`
              (bind _isa (`/Engine/EditorBlueprintResources/StandardMacros.FlipFlop`)
                (:`A`
                  _)
                (:`B`
                  _))
              (`SceneComponent.SetVisibility` (`self.MaterialBillboard1`) _isa true))))
        (:`then_1`
          (if (> (`self.FlipflopTimer`) 1.0)
            (set `self.FlipflopTimer` 0.0)
            (goto _label_3 :!via `Reset`)))))))

(event `/Game/Blueprints/Interfaces/BP_Interact_Interface.Object Interact`
  (`SceneComponent.SetVisibility` (`self.TextRender`) true false)
  (`SceneComponent.SetVisibility` (`self.MaterialBillboard`) true false)
  (set `self.Activate` true)
  (`SceneComponent.SetVisibility` (`self.MaterialBillboard1`) false true)
  (goto _label :!via `Open`))

(event `Reset`)

(event `Hollowlog Cycle`
  (params (NewParam :type "Float (double-precision)"))
  (`KismetSystemLibrary.Delay` NewParam)
  (set `self.LineNumber` (+ 1 (`self.LineNumber`)))
  (goto _label_2 :!via `Reset`))

(fn `Interact with Object Broken`
  (return))

(fn `RotationToPlayer`
  (bind (_returnvalue_roll _returnvalue_pitch _returnvalue_yaw) (`KismetMathLibrary.BreakRotator` (`KismetMathLibrary.FindLookAtRotation` (`self.K2_GetActorLocation`) (`self.K2_GetActorLocation` (cast `/Game/Blueprints/Character/BP_Scout_C` (`GameplayStatics.GetPlayerPawn` 0) :!pure true)))))
  (`SceneComponent.K2_SetWorldRotation` (`self.TextRender`) (`KismetMathLibrary.MakeRotator` 0.0 0.0 _returnvalue_yaw) false false))

(fn `UserConstructionScript`)