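; BP_SoundBox is a trigger box that selects which music BP_Scout uses.
; When a BP_Scout begins overlapping it, the box writes its SongNumber into that Scout's MusicSelect.
; Shortly after BeginPlay, a delayed check applies the same value to the first Scout already overlapping the box, covering a Scout that starts inside it.
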(event `self.ReceiveBeginPlay`
  (bind _output (`|GetArrayItem` (`self.GetOverlappingActors` "/Game/Blueprints/Character/BP_Scout_C.BP_Scout_C_C")))
  (`KismetSystemLibrary.Delay` 0.2)
  (`/Engine/EditorBlueprintResources/StandardMacros.IsValid` _output
    (:`Is Valid`
      (set `/Game/Blueprints/Character/BP_Scout_C.MusicSelect` (`self.SongNumber`) (cast `/Game/Blueprints/Character/BP_Scout_C` _output :!pure true)))))

(event `self.ReceiveActorBeginOverlap`
  (params (OtherActor :type "Actor Object Reference"))
  (bind _asbp_scout_c (cast `/Game/Blueprints/Character/BP_Scout_C` OtherActor))
  (set `/Game/Blueprints/Character/BP_Scout_C.MusicSelect` (`self.SongNumber`) _asbp_scout_c))

(fn `UserConstructionScript`)