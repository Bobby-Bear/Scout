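; BP_HollowLogs is a hollow log object that turns to face the player's BP_Scout pawn.
; BeginPlay opens a Gate after a short delay, letting Tick call RotationToPlayer every frame from then on.
; The rotation takes only the look-at yaw, keeping pitch and roll at zero.
; Its Interact with Object function simply returns false.
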(event `self.ReceiveBeginPlay`
  (`KismetSystemLibrary.Delay` 0.5)
  (goto _label :!via `Open`))

(event `self.ReceiveTick`
  (params (DeltaSeconds :type "Float (single-precision)"))
  (`/Engine/EditorBlueprintResources/StandardMacros.Gate` true :!label _label
    (:`Exit`
      (`self.RotationToPlayer`))))

(fn `Interact with Object`
  (returns (NewParam :type Boolean))
  (return false))

(fn `RotationToPlayer`
  (bind (_returnvalue_roll _returnvalue_pitch _returnvalue_yaw) (`KismetMathLibrary.BreakRotator` (`KismetMathLibrary.FindLookAtRotation` (`self.K2_GetActorLocation`) (`self.K2_GetActorLocation` (cast `/Game/Blueprints/Character/BP_Scout_C` (`GameplayStatics.GetPlayerPawn` 0) :!pure true)))))
  (`self.K2_SetActorRotation` (`KismetMathLibrary.MakeRotator` 0.0 0.0 _returnvalue_yaw)))

(fn `UserConstructionScript`)