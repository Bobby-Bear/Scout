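; Interactable biologist hollow log that plays back a voiced, subtitled recording to the player.
; While idle, it blinks an indicator plane and, until first used, shows the bound Interact key when the player is near.
; Interacting steps through rows of a selected DataTable, timing each line by its sound's duration and resetting when rows run out.
; Text and planes yaw toward the player on Tick.
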(event `self.ReceiveBeginPlay`
  (`SceneComponent.SetVisibility` (`self.TextRender`) false true)
  (`SceneComponent.SetVisibility` (`self.Plane`) false true))

(event `self.ReceiveTick`
  (params (DeltaSeconds :type "Float (single-precision)"))
  (bind (_returnvalue_roll _returnvalue_pitch _returnvalue_yaw) (`KismetMathLibrary.BreakRotator` (`KismetMathLibrary.FindLookAtRotation` (`self.K2_GetActorLocation`) (`self.K2_GetActorLocation` (cast `/Game/Blueprints/Character/BP_Scout_C` (`GameplayStatics.GetPlayerPawn` 0) :!pure true)))))
  (bind (_returnvalue_roll_2 _returnvalue_pitch_2 _returnvalue_yaw_2) (`KismetMathLibrary.BreakRotator` (`KismetMathLibrary.FindLookAtRotation` (`self.K2_GetActorLocation`) (`self.K2_GetActorLocation` (cast `/Game/Blueprints/Character/BP_Scout_C` (`GameplayStatics.GetPlayerPawn` 0) :!pure true)))))
  (`SceneComponent.K2_SetWorldRotation` (`self.Plane1`) (`KismetMathLibrary.MakeRotator` 90.0 0.0 (+ _returnvalue_yaw_2 270.0)) false false)
  (`SceneComponent.K2_SetWorldRotation` (`self.Plane`) (`KismetMathLibrary.MakeRotator` 90.0 0.0 (+ _returnvalue_yaw_2 270.0)) false false)
  (set `self.Delta Seconds` DeltaSeconds)
  (if (`self.Activate`)
    (`/Engine/EditorBlueprintResources/StandardMacros.Gate` true :!label _label
      (:`Exit`
        (`self.RotationToPlayer`)
        (bind _returnvalue (`|GetDataTableRow` (`|GetArrayItem` (`self.HollowLogs DT Array`) (`self.HollowLog Integer`)) (`KismetStringLibrary.Conv_StringToName` (`KismetStringLibrary.Conv_IntToString` (`self.LineNumber`))))
          (:`then`
            (bind (_dialogueline _sound) (break `/Game/Blueprints/Objects/Hollow_Logs/Structure_Hollowlogs` _returnvalue))
            (`TextRenderComponent.K2_SetText` (`self.TextRender`) _dialogueline)
            (`/Engine/EditorBlueprintResources/StandardMacros.DoOnce` false :!label _label_2
              (:`Completed`
                (`GameplayStatics.PlaySound2D` _sound (`/Game/Blueprints/Gamemodes_And_Instances/BP_ScoutInstance_GI.Volume SFX` (cast `/Game/Blueprints/Gamemodes_And_Instances/BP_ScoutInstance_GI` (`GameplayStatics.GetGameInstance`) :!pure true)) 1.0 0.0 null null false)
                (`self.Hollowlog Cycle` (`SoundBase.Duration` _sound)))))
          (:`RowNotFound`
            (`SceneComponent.SetVisibility` (`self.TextRender`) false false)
            (`SceneComponent.SetVisibility` (`self.Plane`) false false)
            (`KismetSystemLibrary.PrintString` "NOOOOOOO")
            (set `self.Activate` false)
            (set `self.LineNumber` 1)
            (goto _label :!via `Close`)))))
    (else
      (`|ExecutionSequence`
        (:`then_0`
          (`/Engine/EditorBlueprintResources/StandardMacros.Gate` false :!label _label_3
            (:`Exit`
              (if (< (`KismetMathLibrary.VSize` (`KismetMathLibrary.Vector_GetAbs` (- (`self.K2_GetActorLocation`) (`self.K2_GetActorLocation` (`GameplayStatics.GetPlayerPawn` 0))))) 1000.0)
                (`TextRenderComponent.K2_SetText` (`self.Text`) (`KismetTextLibrary.Conv_StringToText` (`KismetStringLibrary.Concat_StrStr` (`KismetTextLibrary.Conv_TextToString` "Press \"") (`KismetTextLibrary.Conv_TextToString` (`KismetInputLibrary.Key_GetDisplayName` (`.Key` (break `InputActionKeyMapping` (`|GetArrayItem` (`InputSettings.GetActionMappingByName` (`InputSettings.GetInputSettings`) "Interact")))))) (`KismetTextLibrary.Conv_TextToString` "\" To Interact"))))
                (`SceneComponent.K2_SetWorldRotation` (`self.Text`) (`KismetMathLibrary.MakeRotator` 0.0 0.0 _returnvalue_yaw) false false)
                (`SceneComponent.SetVisibility` (`self.Text`) true false)
                (else
                  (`SceneComponent.SetVisibility` (`self.Text`) false false))))))
        (:`then_1`
          (set `self.FlipflopTimer` (+ (`self.Delta Seconds`) (`self.FlipflopTimer`)))
          (`|ExecutionSequence`
            (:`then_0`
              (`/Engine/EditorBlueprintResources/StandardMacros.DoOnce` false :!label _label_4
                (:`Completed`
                  (bind _isa (`/Engine/EditorBlueprintResources/StandardMacros.FlipFlop`)
                    (:`A`
                      _)
                    (:`B`
                      _))
                  (`SceneComponent.SetVisibility` (`self.Plane1`) _isa true))))
            (:`then_1`
              (if (> (`self.FlipflopTimer`) 0.25)
                (set `self.FlipflopTimer` 0.0)
                (goto _label_4 :!via `Reset`)))))))))

(event `/Game/Blueprints/Interfaces/BP_Interact_Interface.Object Interact`
  (`SceneComponent.SetVisibility` (`self.TextRender`) true false)
  (`SceneComponent.SetVisibility` (`self.Plane`) true false)
  (set `self.Activate` true)
  (`SceneComponent.SetVisibility` (`self.Plane1`) false true)
  (`|ExecutionSequence`
    (:`then_0`
      (`GameplayStatics.PlaySound2D` "/Engine/EditorSounds/Notifications/CompileFailed.CompileFailed" (`/Game/Blueprints/Gamemodes_And_Instances/BP_ScoutInstance_GI.Volume SFX` (cast `/Game/Blueprints/Gamemodes_And_Instances/BP_ScoutInstance_GI` (`GameplayStatics.GetGameInstance`) :!pure true)) 1.0 0.0 null null)
      (`KismetSystemLibrary.Delay` 0.2)
      (goto _label :!via `Open`))
    (:`then_1`
      (`SceneComponent.SetVisibility` (`self.Text`) false false)
      (goto _label_3 :!via `Close`))))

(event `Hollowlog Cycle`
  (params (NewParam :type "Float (double-precision)"))
  (`KismetSystemLibrary.Delay` NewParam)
  (`KismetSystemLibrary.Delay` 0.1)
  (set `self.LineNumber` (+ 1 (`self.LineNumber`)))
  (goto _label_2 :!via `Reset`))

(fn `Interact with Object Broken`
  (return))

(fn `RotationToPlayer`
  (bind (_returnvalue_roll _returnvalue_pitch _returnvalue_yaw) (`KismetMathLibrary.BreakRotator` (`KismetMathLibrary.FindLookAtRotation` (`self.K2_GetActorLocation`) (`self.K2_GetActorLocation` (cast `/Game/Blueprints/Character/BP_Scout_C` (`GameplayStatics.GetPlayerPawn` 0) :!pure true)))))
  (`SceneComponent.K2_SetWorldRotation` (`self.TextRender`) (`KismetMathLibrary.MakeRotator` 0.0 0.0 _returnvalue_yaw) false false))

(fn `UserConstructionScript`)