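; BP_SaveBox is a checkpoint trigger that saves the game when the Scout player overlaps it.
; After a one-second delay, it copies the player pawn's location, camera yaw and collected boots, grappling hook and key card states into the game instance as respawn data.
; It then calls UpdateSave on the Scout testing game mode.
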(event `self.ReceiveBeginPlay`)

(event `self.ReceiveActorBeginOverlap`
  (params (OtherActor :type "Actor Object Reference"))
  (bind _asbp_scout_instance_gi (cast `/Game/Blueprints/Gamemodes_And_Instances/BP_ScoutInstance_GI` (`GameplayStatics.GetGameInstance`) :!pure true))
  (bind _asbp_scout_c (cast `/Game/Blueprints/Character/BP_Scout_C` (`GameplayStatics.GetPlayerPawn` 0) :!pure true))
  (`KismetSystemLibrary.Delay` 1.0)
  (cast `/Game/Blueprints/Character/BP_Scout_C` OtherActor)
  (`/Engine/EditorBlueprintResources/StandardMacros.IsValid` _asbp_scout_c
    (:`Is Valid`
      (set `/Game/Blueprints/Gamemodes_And_Instances/BP_ScoutInstance_GI.LocationSpawnNew` (`self.K2_GetActorLocation` _asbp_scout_c) _asbp_scout_instance_gi)
      (set `/Game/Blueprints/Gamemodes_And_Instances/BP_ScoutInstance_GI.RotationSpawnNew` (`/Game/Blueprints/Character/BP_Scout_C.CameraRotationYaw` _asbp_scout_c) _asbp_scout_instance_gi)
      (set `/Game/Blueprints/Gamemodes_And_Instances/BP_ScoutInstance_GI.BootsCollected` (`/Game/Blueprints/Character/BP_Scout_C.BootsCollected` _asbp_scout_c) _asbp_scout_instance_gi)
      (set `/Game/Blueprints/Gamemodes_And_Instances/BP_ScoutInstance_GI.GrapplingHookCollected` (`/Game/Blueprints/Character/BP_Scout_C.GrapplingHookCollected` _asbp_scout_c) _asbp_scout_instance_gi)
      (set `/Game/Blueprints/Gamemodes_And_Instances/BP_ScoutInstance_GI.KeyCardCollected` (`/Game/Blueprints/Character/BP_Scout_C.KeyCardCollected` _asbp_scout_c) _asbp_scout_instance_gi)
      (`/Game/Blueprints/Gamemodes_And_Instances/BP_ScoutTesting_GM.Update Save` (cast `/Game/Blueprints/Gamemodes_And_Instances/BP_ScoutTesting_GM` (`GameplayStatics.GetGameMode`) :!pure true)))))

(fn `UserConstructionScript`)