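; BP_Artifact is an interactable artifact that the player's scout collects and carries in view.
; Interacting spawns a BP_Robot nearby linked to the artifact and flagged RobotEnd, notifies BP_Scout of collection, disables mesh collision and halves the artifact's scale.
; It also opens a Gate, through which Tick sweeps the artifact to an offset in front of the player camera each frame while RobotGiven is false.
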(event `/Game/Blueprints/Interfaces/BP_Interact_Interface.Object Interact`
  (bind _asbp_scout_c (cast `/Game/Blueprints/Character/BP_Scout_C` (`GameplayStatics.GetPlayerPawn` 0) :!pure true))
  (bind _camera (`/Game/Blueprints/Character/BP_Scout_C.Camera` _asbp_scout_c))
  (bind _returnvalue (`|SpawnActorFromClass` "/Game/Blueprints/Objects/BP_Robot.BP_Robot_C" (`KismetMathLibrary.MakeTransform` (`KismetMathLibrary.MakeVector` (+ (.x (`self.K2_GetActorLocation`)) 100.0) (.y (`self.K2_GetActorLocation`)) (.z (`self.K2_GetActorLocation`)))) "Undefined" "OverrideRootScale" null null))
  (set `/Game/Blueprints/Objects/BP_Robot.Artifact` self _returnvalue)
  (set `/Game/Blueprints/Objects/BP_Robot.RobotEnd` true _returnvalue)
  (set `self.Robot` _returnvalue)
  (`PrimitiveComponent.SetCollisionEnabled` (`self.SM_Artifact`) "NoCollision")
  (`PrimitiveComponent.SetCollisionEnabled` (`self.SM_ArtifactCapsule`) "NoCollision")
  (`/Game/Blueprints/Character/BP_Scout_C.Artifact Collected` _asbp_scout_c)
  (`self.SetActorScale3D` (* (`self.GetActorScale3D`) 0.5))
  (goto _label :!via `Open`))

(event `self.ReceiveTick`
  (params (DeltaSeconds :type "Float (single-precision)"))
  (bind _camera (`/Game/Blueprints/Character/BP_Scout_C.Camera` (cast `/Game/Blueprints/Character/BP_Scout_C` (`GameplayStatics.GetPlayerPawn` 0) :!pure true)))
  (if (not (`self.RobotGiven`))
    (`/Engine/EditorBlueprintResources/StandardMacros.Gate` true :!label _label
      (:`Exit`
        (`self.K2_SetActorLocation` (+ (`SceneComponent.K2_GetComponentLocation` _camera) (* (`KismetMathLibrary.GetForwardVector` (`KismetMathLibrary.MakeRotator` (+ (.roll (`SceneComponent.K2_GetComponentRotation` _camera)) -30.0) (+ (.pitch (`SceneComponent.K2_GetComponentRotation` _camera)) -30.0) (+ (.yaw (`SceneComponent.K2_GetComponentRotation` _camera)) -30.0))) 50.0)) true)))))

(fn `UserConstructionScript`)