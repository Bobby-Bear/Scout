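; Interactable ship manual book that shows its UI when the player interacts with it.
; Each tick, within a fixed range of the player pawn, it shows an "Interact" prompt with the bound key's name, yawed toward the BP_Scout player; otherwise the prompt is hidden.
; ObjectInteract prints a debug string, adds a book fade widget to the viewport, then after a short delay adds the manual widget.
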(event `self.ReceiveTick`
  (params (DeltaSeconds :type "Float (single-precision)"))
  (bind (_returnvalue_roll _returnvalue_pitch _returnvalue_yaw) (`KismetMathLibrary.BreakRotator` (`KismetMathLibrary.FindLookAtRotation` (`self.K2_GetActorLocation`) (`self.K2_GetActorLocation` (cast `/Game/Blueprints/Character/BP_Scout_C` (`GameplayStatics.GetPlayerPawn` 0) :!pure true)))))
  (if (< (`KismetMathLibrary.VSize` (`KismetMathLibrary.Vector_GetAbs` (- (`self.K2_GetActorLocation`) (`self.K2_GetActorLocation` (`GameplayStatics.GetPlayerPawn` 0))))) 1000.0)
    (`TextRenderComponent.K2_SetText` (`self.Text`) (`KismetTextLibrary.Conv_StringToText` (`KismetStringLibrary.Concat_StrStr` (`KismetTextLibrary.Conv_TextToString` "Press \"") (`KismetTextLibrary.Conv_TextToString` (`KismetInputLibrary.Key_GetDisplayName` (`.Key` (break `InputActionKeyMapping` (`|GetArrayItem` (`InputSettings.GetActionMappingByName` (`InputSettings.GetInputSettings`) "Interact")))))) (`KismetTextLibrary.Conv_TextToString` "\" To Interact"))))
    (`SceneComponent.K2_SetWorldRotation` (`self.Text`) (`KismetMathLibrary.MakeRotator` 0.0 0.0 _returnvalue_yaw) false false)
    (`SceneComponent.SetVisibility` (`self.Text`) true false)
    (else
      (`SceneComponent.SetVisibility` (`self.Text`) false false))))

(event `/Game/Blueprints/Interfaces/BP_Interact_Interface.Object Interact`
  (bind _returnvalue (`GameplayStatics.GetPlayerController` 0))
  (`KismetSystemLibrary.PrintString` "Hello")
  (bind _returnvalue_2 (`|CreateWidget` "/Game/Blueprints/Widgets/Transitions/Bp_BookFade_Widget.Bp_BookFade_Widget_C" _returnvalue))
  (`UserWidget.AddToViewport` _returnvalue_2 0)
  (`KismetSystemLibrary.Delay` 0.2)
  (bind _returnvalue_3 (`|CreateWidget` "/Game/Blueprints/Objects/Books/ShipManual/BP_ShipManual_Widget1.BP_ShipManual_Widget1_C" _returnvalue))
  (`UserWidget.AddToViewport` _returnvalue_3 0))

(fn `UserConstructionScript`)