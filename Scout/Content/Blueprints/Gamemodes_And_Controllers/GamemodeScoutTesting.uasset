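; Scout testing game mode that creates and saves the player's spawn checkpoint through a SaveState object held on ScoutGameInstance.
; Shortly after BeginPlay it calls UpdateSave if no save state exists in memory, seeding it with default start location and rotation.
; Later UpdateSave calls copy the game instance's new spawn transform and write to slot.
; Load moves the player to the in-memory saved location; its subsequent slot read is unused.
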(event `self.ReceiveBeginPlay`
  (`KismetSystemLibrary.Delay` 0.2)
  (`/Engine/EditorBlueprintResources/StandardMacros.IsValid` (`/Game/Blueprints/Gamemodes_And_Controllers/ScoutGameInstance.SaveState Instance` (cast `/Game/Blueprints/Gamemodes_And_Controllers/ScoutGameInstance` (`GameplayStatics.GetGameInstance`) :!pure true))
    (:`Is Valid`
      (`KismetSystemLibrary.PrintString` "STATE EXISTS"))
    (:`Is Not Valid`
      (`self.Update Save`))))

(event `Load`
  (`self.K2_SetActorLocation` (`GameplayStatics.GetPlayerPawn` 0) (`/Game/Blueprints/Gamemodes_And_Controllers/SaveState.SaveLocation` (`/Game/Blueprints/Gamemodes_And_Controllers/ScoutGameInstance.SaveState Instance` (cast `/Game/Blueprints/Gamemodes_And_Controllers/ScoutGameInstance` (`GameplayStatics.GetGameInstance`) :!pure true))) false false)
  (`KismetSystemLibrary.PrintString` "Loaded")
  (`GameplayStatics.LoadGameFromSlot` (`self.Gamemode Slot Name`)))

(event `Update Save`
  (bind _asscout_game_instance (cast `/Game/Blueprints/Gamemodes_And_Controllers/ScoutGameInstance` (`GameplayStatics.GetGameInstance`) :!pure true))
  (bind _asscout_game_instance_2 (cast `/Game/Blueprints/Gamemodes_And_Controllers/ScoutGameInstance` (`GameplayStatics.GetGameInstance`) :!pure true))
  (bind _savestate_instance (`/Game/Blueprints/Gamemodes_And_Controllers/ScoutGameInstance.SaveState Instance` _asscout_game_instance))
  (bind _savestate_instance_2 (`/Game/Blueprints/Gamemodes_And_Controllers/ScoutGameInstance.SaveState Instance` _asscout_game_instance_2))
  (`/Engine/EditorBlueprintResources/StandardMacros.IsValid` (`/Game/Blueprints/Gamemodes_And_Controllers/ScoutGameInstance.SaveState Instance` (cast `/Game/Blueprints/Gamemodes_And_Controllers/ScoutGameInstance` (`GameplayStatics.GetGameInstance`) :!pure true))
    (:`Is Valid`
      (set `/Game/Blueprints/Gamemodes_And_Controllers/SaveState.SaveLocation` (`/Game/Blueprints/Gamemodes_And_Controllers/ScoutGameInstance.LocationSpawnNew` _asscout_game_instance_2) _savestate_instance_2)
      (set `/Game/Blueprints/Gamemodes_And_Controllers/SaveState.SaveRotation` (`/Game/Blueprints/Gamemodes_And_Controllers/ScoutGameInstance.RotationSpawnNew` _asscout_game_instance_2) _savestate_instance_2))
    (:`Is Not Valid`
      (bind _returnvalue (`GameplayStatics.CreateSaveGameObject` "/Game/Blueprints/Gamemodes_And_Controllers/SaveState.SaveState_C"))
      (set `/Game/Blueprints/Gamemodes_And_Controllers/ScoutGameInstance.SaveState Instance` _returnvalue _asscout_game_instance)
      (set `/Game/Blueprints/Gamemodes_And_Controllers/SaveState.SaveLocation` (`self.PlayerLocationStart Default`) _savestate_instance)
      (set `/Game/Blueprints/Gamemodes_And_Controllers/SaveState.SaveRotation` (`self.PlayerRotationStart Default`) _savestate_instance)))
  (`GameplayStatics.SaveGameToSlot` _savestate_instance (`/Game/Blueprints/Gamemodes_And_Controllers/SaveState.SaveSlotName` _savestate_instance) (`/Game/Blueprints/Gamemodes_And_Controllers/SaveState.UserIndex` _savestate_instance))
  (`KismetSystemLibrary.PrintString` (`KismetStringLibrary.Conv_VectorToString` (`/Game/Blueprints/Gamemodes_And_Controllers/SaveState.SaveLocation` _savestate_instance))))

(fn `UserConstructionScript`)