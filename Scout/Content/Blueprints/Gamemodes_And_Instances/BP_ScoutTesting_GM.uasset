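; Scout testing game mode that manages saving and loading of player position, camera yaw, pickups and settings.
; BeginPlay creates a default BP_SaveState_SG if the game instance holds none.
; UpdateSave and SaveSettings copy game-instance values into it and write to slot, sharing most steps; Load and LoadSettings copy them back to the instance, with Load also updating the pawn.
; Any key press also feeds the control-rebinding widget when SetControl is set.
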(event `Key|AnyKey`
  (params (Key :type "Key Structure"))
  (bind _setcontrolswidget (`self.SetControlsWidget`))
  (:`Pressed`
    (`KismetSystemLibrary.PrintString` "Hello")
    (if (`self.SetControl`)
      (set `/Game/Blueprints/Widgets/Menus/Settings_Widgets/BP_SetControl_Widget.Key Pressed` Key _setcontrolswidget)
      (`/Game/Blueprints/Widgets/Menus/Settings_Widgets/BP_SetControl_Widget.Button Pressed` _setcontrolswidget))))

(event `self.ReceiveBeginPlay`
  (`KismetSystemLibrary.Delay` 0.2)
  (`/Engine/EditorBlueprintResources/StandardMacros.IsValid` (`/Game/Blueprints/Gamemodes_And_Instances/BP_ScoutInstance_GI.SaveState Instance` (cast `/Game/Blueprints/Gamemodes_And_Instances/BP_ScoutInstance_GI` (`GameplayStatics.GetGameInstance`) :!pure true))
    (:`Is Valid`
      (`KismetSystemLibrary.PrintString` "STATE EXISTS"))
    (:`Is Not Valid`
      (`self.Update Save`))))

(event `Load Settings`
  (bind _asbp_scout_instance_gi (cast `/Game/Blueprints/Gamemodes_And_Instances/BP_ScoutInstance_GI` (`GameplayStatics.GetGameInstance`) :!pure true))
  (bind _savestate_instance (`/Game/Blueprints/Gamemodes_And_Instances/BP_ScoutInstance_GI.SaveState Instance` _asbp_scout_instance_gi))
  (set `/Game/Blueprints/Gamemodes_And_Instances/BP_ScoutInstance_GI.Sensitivity` (`/Game/Blueprints/Gamemodes_And_Instances/BP_SaveState_SG.SaveSensitivity` _savestate_instance) _asbp_scout_instance_gi :!label _label)
  (set `/Game/Blueprints/Gamemodes_And_Instances/BP_ScoutInstance_GI.Volume Music` (`/Game/Blueprints/Gamemodes_And_Instances/BP_SaveState_SG.SaveMusic` _savestate_instance) _asbp_scout_instance_gi)
  (set `/Game/Blueprints/Gamemodes_And_Instances/BP_ScoutInstance_GI.Volume SFX` (`/Game/Blueprints/Gamemodes_And_Instances/BP_SaveState_SG.SaveSFX` _savestate_instance) _asbp_scout_instance_gi)
  (set `/Game/Blueprints/Gamemodes_And_Instances/BP_ScoutInstance_GI.GraphicsQuality` (`/Game/Blueprints/Gamemodes_And_Instances/BP_SaveState_SG.GraphicsQuality` _savestate_instance) _asbp_scout_instance_gi)
  (`KismetSystemLibrary.PrintString` "Loaded")
  (`GameplayStatics.LoadGameFromSlot` (`self.Gamemode Slot Name`)))

(event `Load`
  (bind _asbp_scout_c (cast `/Game/Blueprints/Character/BP_Scout_C` (`GameplayStatics.GetPlayerPawn` 0) :!pure true))
  (bind _asbp_scout_instance_gi (cast `/Game/Blueprints/Gamemodes_And_Instances/BP_ScoutInstance_GI` (`GameplayStatics.GetGameInstance`) :!pure true))
  (bind _savestate_instance (`/Game/Blueprints/Gamemodes_And_Instances/BP_ScoutInstance_GI.SaveState Instance` _asbp_scout_instance_gi))
  (`self.K2_SetActorLocation` _asbp_scout_c (`/Game/Blueprints/Gamemodes_And_Instances/BP_SaveState_SG.SaveLocation` _savestate_instance) false false)
  (set `/Game/Blueprints/Character/BP_Scout_C.CameraRotationYaw` (`/Game/Blueprints/Gamemodes_And_Instances/BP_SaveState_SG.SaveRotation` _savestate_instance) _asbp_scout_c)
  (bind _output_get (set `/Game/Blueprints/Gamemodes_And_Instances/BP_ScoutInstance_GI.BootsCollected` (`/Game/Blueprints/Gamemodes_And_Instances/BP_SaveState_SG.Boots` _savestate_instance) _asbp_scout_instance_gi))
  (bind _output_get_2 (set `/Game/Blueprints/Gamemodes_And_Instances/BP_ScoutInstance_GI.GrapplingHookCollected` (`/Game/Blueprints/Gamemodes_And_Instances/BP_SaveState_SG.GrapplingHook` _savestate_instance) _asbp_scout_instance_gi))
  (bind _output_get_3 (set `/Game/Blueprints/Gamemodes_And_Instances/BP_ScoutInstance_GI.KeyCardCollected` (`/Game/Blueprints/Gamemodes_And_Instances/BP_SaveState_SG.KeyCard` _savestate_instance) _asbp_scout_instance_gi))
  (`|ExecutionSequence`
    (:`then_0`
      (set `/Game/Blueprints/Character/BP_Scout_C.BootsCollected` _output_get _asbp_scout_c)
      (set `/Game/Blueprints/Character/BP_Scout_C.GrapplingHookCollected` _output_get_2 _asbp_scout_c)
      (set `/Game/Blueprints/Character/BP_Scout_C.KeyCardCollected` _output_get_3 _asbp_scout_c))
    (:`then_1`
      (goto _label))))

(event `Update Save`
  (bind _asbp_scout_instance_gi (cast `/Game/Blueprints/Gamemodes_And_Instances/BP_ScoutInstance_GI` (`GameplayStatics.GetGameInstance`) :!pure true))
  (bind _asbp_scout_instance_gi_2 (cast `/Game/Blueprints/Gamemodes_And_Instances/BP_ScoutInstance_GI` (`GameplayStatics.GetGameInstance`) :!pure true))
  (bind _savestate_instance (`/Game/Blueprints/Gamemodes_And_Instances/BP_ScoutInstance_GI.SaveState Instance` _asbp_scout_instance_gi))
  (bind _savestate_instance_2 (`/Game/Blueprints/Gamemodes_And_Instances/BP_ScoutInstance_GI.SaveState Instance` _asbp_scout_instance_gi_2))
  (bind _bootscollected (`/Game/Blueprints/Gamemodes_And_Instances/BP_ScoutInstance_GI.BootsCollected` _asbp_scout_instance_gi_2))
  (`/Engine/EditorBlueprintResources/StandardMacros.IsValid` (`/Game/Blueprints/Gamemodes_And_Instances/BP_ScoutInstance_GI.SaveState Instance` (cast `/Game/Blueprints/Gamemodes_And_Instances/BP_ScoutInstance_GI` (`GameplayStatics.GetGameInstance`) :!pure true))
    (:`Is Valid`
      (set `/Game/Blueprints/Gamemodes_And_Instances/BP_SaveState_SG.SaveLocation` (`/Game/Blueprints/Gamemodes_And_Instances/BP_ScoutInstance_GI.LocationSpawnNew` _asbp_scout_instance_gi_2) _savestate_instance_2)
      (set `/Game/Blueprints/Gamemodes_And_Instances/BP_SaveState_SG.SaveRotation` (`/Game/Blueprints/Gamemodes_And_Instances/BP_ScoutInstance_GI.RotationSpawnNew` _asbp_scout_instance_gi_2) _savestate_instance_2)
      (set `/Game/Blueprints/Gamemodes_And_Instances/BP_SaveState_SG.SaveMusic` (`/Game/Blueprints/Gamemodes_And_Instances/BP_ScoutInstance_GI.Volume Music` _asbp_scout_instance_gi_2) _savestate_instance_2 :!label _label_2)
      (set `/Game/Blueprints/Gamemodes_And_Instances/BP_SaveState_SG.SaveSFX` (`/Game/Blueprints/Gamemodes_And_Instances/BP_ScoutInstance_GI.Volume SFX` _asbp_scout_instance_gi_2) _savestate_instance_2)
      (set `/Game/Blueprints/Gamemodes_And_Instances/BP_SaveState_SG.SaveSensitivity` (`/Game/Blueprints/Gamemodes_And_Instances/BP_ScoutInstance_GI.Sensitivity` _asbp_scout_instance_gi_2) _savestate_instance_2)
      (set `/Game/Blueprints/Gamemodes_And_Instances/BP_SaveState_SG.Boots` _bootscollected _savestate_instance_2)
      (`KismetSystemLibrary.PrintString` (`KismetStringLibrary.Conv_BoolToString` _bootscollected))
      (set `/Game/Blueprints/Gamemodes_And_Instances/BP_SaveState_SG.GrapplingHook` (`/Game/Blueprints/Gamemodes_And_Instances/BP_ScoutInstance_GI.GrapplingHookCollected` _asbp_scout_instance_gi_2) _savestate_instance_2)
      (set `/Game/Blueprints/Gamemodes_And_Instances/BP_SaveState_SG.KeyCard` (`/Game/Blueprints/Gamemodes_And_Instances/BP_ScoutInstance_GI.KeyCardCollected` _asbp_scout_instance_gi_2) _savestate_instance_2)
      (set `/Game/Blueprints/Gamemodes_And_Instances/BP_SaveState_SG.GraphicsQuality` (`/Game/Blueprints/Gamemodes_And_Instances/BP_ScoutInstance_GI.GraphicsQuality` _asbp_scout_instance_gi_2) _savestate_instance_2))
    (:`Is Not Valid`
      (bind _returnvalue (`GameplayStatics.CreateSaveGameObject` "/Game/Blueprints/Gamemodes_And_Instances/BP_SaveState_SG.BP_SaveState_SG_C"))
      (set `/Game/Blueprints/Gamemodes_And_Instances/BP_ScoutInstance_GI.SaveState Instance` _returnvalue _asbp_scout_instance_gi)
      (set `/Game/Blueprints/Gamemodes_And_Instances/BP_SaveState_SG.SaveLocation` (`self.PlayerLocationStart Default`) _savestate_instance)
      (set `/Game/Blueprints/Gamemodes_And_Instances/BP_SaveState_SG.SaveRotation` (`self.PlayerRotationStart Default`) _savestate_instance :!label _label_3)
      (set `/Game/Blueprints/Gamemodes_And_Instances/BP_SaveState_SG.SaveMusic` (`self.Music Default`) _savestate_instance)
      (set `/Game/Blueprints/Gamemodes_And_Instances/BP_SaveState_SG.SaveSFX` (`self.SFX Default`) _savestate_instance)
      (set `/Game/Blueprints/Gamemodes_And_Instances/BP_SaveState_SG.SaveSensitivity` (`self.Sensitivity Default`) _savestate_instance)
      (set `/Game/Blueprints/Gamemodes_And_Instances/BP_SaveState_SG.Boots` false _savestate_instance)
      (set `/Game/Blueprints/Gamemodes_And_Instances/BP_SaveState_SG.GrapplingHook` false _savestate_instance)
      (set `/Game/Blueprints/Gamemodes_And_Instances/BP_SaveState_SG.KeyCard` false _savestate_instance)
      (set `/Game/Blueprints/Gamemodes_And_Instances/BP_SaveState_SG.GraphicsQuality` 3 _savestate_instance)))
  (`GameplayStatics.SaveGameToSlot` _savestate_instance (`/Game/Blueprints/Gamemodes_And_Instances/BP_SaveState_SG.SaveSlotName` _savestate_instance) (`/Game/Blueprints/Gamemodes_And_Instances/BP_SaveState_SG.UserIndex` _savestate_instance))
  (`KismetSystemLibrary.PrintString` (`KismetStringLibrary.Conv_VectorToString` (`/Game/Blueprints/Gamemodes_And_Instances/BP_SaveState_SG.SaveLocation` _savestate_instance)))
  (`KismetSystemLibrary.PrintString` (`KismetStringLibrary.Conv_RotatorToString` (`/Game/Blueprints/Gamemodes_And_Instances/BP_SaveState_SG.SaveRotation` _savestate_instance))))

(event `Save Settings`
  (`/Engine/EditorBlueprintResources/StandardMacros.IsValid` (`/Game/Blueprints/Gamemodes_And_Instances/BP_ScoutInstance_GI.SaveState Instance` (cast `/Game/Blueprints/Gamemodes_And_Instances/BP_ScoutInstance_GI` (`GameplayStatics.GetGameInstance`) :!pure true))
    (:`Is Valid`
      (goto _label_2))
    (:`Is Not Valid`
      (`GameplayStatics.CreateSaveGameObject` "/Game/Blueprints/Gamemodes_And_Instances/BP_SaveState_SG.BP_SaveState_SG_C")
      (goto _label_3))))

(fn `Make Keys Array`
  (locals (InputArray :type "Array of Text"))
  (bind _returnvalue (`InputSettings.GetInputSettings`))
  (for _array_element (`InputSettings.GetActionNames` _returnvalue)
    (for _array_element_2 (`InputSettings.GetActionMappingByName` _returnvalue _array_element)
      (`KismetArrayLibrary.Array_Add` (`self.Array`) (`.Key` (break `InputActionKeyMapping` _array_element_2)))))
  (for _ (`InputSettings.GetAxisNames` _returnvalue)
    (for _array_element_3 (`InputSettings.GetAxisMappingByName` _returnvalue "None")
      (`KismetArrayLibrary.Array_Add` (`self.Array`) (`.Key` (break `InputAxisKeyMapping` _array_element_3)))
      (`KismetSystemLibrary.PrintString` "1Hello"))))

(fn `UserConstructionScript`)