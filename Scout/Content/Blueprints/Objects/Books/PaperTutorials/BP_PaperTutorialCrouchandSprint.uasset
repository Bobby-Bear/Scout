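; Interactable paper that opens the crouch tutorial (crouch and sprint, per the asset name).
; Every Tick, a text prompt shows the bound Interact key and yaws toward the player's BP_Scout when within 2000 units, hiding otherwise.
; On ObjectInteract, it disables player pawn input and adds a book-fade widget and the crouch tutorial widget to the viewport.
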(event `self.ReceiveTick`
  (params (DeltaSeconds :type "Float (single-precision)"))
  (bind (_returnvalue_roll _returnvalue_pitch _returnvalue_yaw) (`KismetMathLibrary.BreakRotator` (`KismetMathLibrary.FindLookAtRotation` (`self.K2_GetActorLocation`) (`self.K2_GetActorLocation` (cast `/Game/Blueprints/Character/BP_Scout_C` (`GameplayStatics.GetPlayerPawn` 0) :!pure true)))))
  (if (< (`KismetMathLibrary.VSize` (`KismetMathLibrary.Vector_GetAbs` (- (`self.K2_GetActorLocation`) (`self.K2_GetActorLocation` (`GameplayStatics.GetPlayerPawn` 0))))) 2000.0)
    (`TextRenderComponent.K2_SetText` (`self.Text`) (`KismetTextLibrary.Conv_StringToText` (`KismetStringLibrary.Concat_StrStr` (`KismetTextLibrary.Conv_TextToString` "Press \"") (`KismetTextLibrary.Conv_TextToString` (`KismetInputLibrary.Key_GetDisplayName` (`.Key` (break `InputActionKeyMapping` (`|GetArrayItem` (`InputSettings.GetActionMappingByName` (`InputSettings.GetInputSettings`) "Interact")))))) (`KismetTextLibrary.Conv_TextToString` "\" To Interact"))))
    (`SceneComponent.K2_SetWorldRotation` (`self.Text`) (`KismetMathLibrary.MakeRotator` 0.0 0.0 _returnvalue_yaw) false false)
    (`SceneComponent.SetVisibility` (`self.Text`) true false)
    (else
      (`SceneComponent.SetVisibility` (`self.Text`) false false))))

(event `/Game/Blueprints/Interfaces/BP_Interact_Interface.Object Interact`
  (bind _returnvalue (`GameplayStatics.GetPlayerController` 0))
  (bind _returnvalue_2 (`|CreateWidget` "/Game/Blueprints/Widgets/Transitions/Bp_BookFade_Widget.Bp_BookFade_Widget_C" _returnvalue))
  (`self.DisableInput` (`GameplayStatics.GetPlayerPawn` 0) _returnvalue)
  (bind _returnvalue_3 (`|CreateWidget` "/Game/Blueprints/Objects/Books/PaperTutorials/PaperWidgets/BP_PaperTutorialsCrouch_Widget.BP_PaperTutorialsCrouch_Widget_C" (`GameplayStatics.GetPlayerController` 0)))
  (`UserWidget.AddToViewport` _returnvalue_2 0)
  (`UserWidget.AddToViewport` _returnvalue_3 0))

(fn `UserConstructionScript`)